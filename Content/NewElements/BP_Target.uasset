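; BP_Target is a shootable target actor that takes damage from first-person projectile hits and explodes when its health runs out.
; Each projectile hit spawns a sparks effect at the impact point, stores it in an array and applies fixed damage to itself.
; At zero health it destroys its mesh, then loops over the sparks, removing each and spawning an explosion, with a Delay inside the loop before destroying explosion and target.
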(event `self.ReceiveAnyDamage`
  (params (Damage :type "Float (single-precision)") (DamageType :type "DamageType Object Reference") (InstigatedBy :type "Controller Object Reference") (DamageCauser :type "Actor Object Reference"))
  (bind _health (`self.health`))
  ;[1 1 1] take damage
  (set `self.health` (- _health Damage))
  (if (<= _health 0.0)
    (`ActorComponent.K2_DestroyComponent` (`self.StaticMesh`))
    (for _array_element (`self.sparksArray`)
      (`self.K2_DestroyActor` _array_element)
      (bind _returnvalue (`|SpawnActorFromClass` "/Game/StarterContent/Blueprints/Blueprint_Effect_Explosion.Blueprint_Effect_Explosion_C" (`KismetMathLibrary.Conv_VectorToTransform` (`self.K2_GetActorLocation`)) "AlwaysSpawn" "OverrideRootScale" null null))
      (`KismetSystemLibrary.Delay` 0.5)
      (`self.K2_DestroyActor` _returnvalue)
      (`self.K2_DestroyActor`))))

(event `self.ReceiveHit`
  (params (MyComp :type "PrimitiveComponent Object Reference") (Other :type "Actor Object Reference") (OtherComp :type "PrimitiveComponent Object Reference") (bSelfMoved :type Boolean) (HitLocation :type "Vector Structure") (HitNormal :type "Vector Structure") (NormalImpulse :type "Vector Structure") (Hit :type "HitResult Structure (by ref)"))
  ;[1 1 1] hit
  (cast `/Game/FirstPerson/Blueprints/BP_FirstPersonProjectile` Other)
  (bind _returnvalue (`|SpawnActorFromClass` "/Game/StarterContent/Blueprints/Blueprint_Effect_Sparks.Blueprint_Effect_Sparks_C" (`KismetMathLibrary.Conv_VectorToTransform` HitLocation) "AlwaysSpawn" "OverrideRootScale" null null))
  (`|ExecutionSequence`
    (:`then_0`
      (`KismetArrayLibrary.Array_Set` (`self.sparksArray`) (`KismetArrayLibrary.Array_Length` (`self.sparksArray`)) _returnvalue true))
    (:`then_1`
      (`GameplayStatics.ApplyDamage` self 25.0))))

(fn `UserConstructionScript`)