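; BP_hazard is a hazard actor that hurts and bounces the first-person player character on contact.
; On BeginPlay it spawns an actor of the same class as its Flames reference at its own location.
; When hit by BP_FirstPersonCharacter, it spawns an explosion effect at the hit point, applies damage and launches the character upward.
; Hits from any other actor are ignored.
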(event `self.ReceiveBeginPlay`
  (`|SpawnActorFromClass` (`GameplayStatics.GetObjectClass` (`self.flames`)) (`KismetMathLibrary.Conv_VectorToTransform` (`self.K2_GetActorLocation` self)) "Undefined" "OverrideRootScale" null null))

(event `self.ReceiveHit`
  (params (MyComp :type "PrimitiveComponent Object Reference") (Other :type "Actor Object Reference") (OtherComp :type "PrimitiveComponent Object Reference") (bSelfMoved :type Boolean) (HitLocation :type "Vector Structure") (HitNormal :type "Vector Structure") (NormalImpulse :type "Vector Structure") (Hit :type "HitResult Structure (by ref)"))
  (bind _asbp_first_person_character (cast `/Game/FirstPerson/Blueprints/BP_FirstPersonCharacter` Other))
  (`|SpawnActorFromClass` "/Game/StarterContent/Blueprints/Blueprint_Effect_Explosion.Blueprint_Effect_Explosion_C" (`KismetMathLibrary.Conv_VectorToTransform` HitLocation) "Undefined" "OverrideRootScale" null null)
  (`GameplayStatics.ApplyDamage` _asbp_first_person_character 10.0)
  (`Character.LaunchCharacter` _asbp_first_person_character (+ (0.0 0.0 0.0) (0.0 0.0 300.0)) false false))

(fn `UserConstructionScript`)